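; Player character with twin-stick style controls: world-axis movement and aim input that turns and fires.
; Both aim axes share one path that lerps control rotation toward the input direction at a delta-time-scaled turn rate.
; While aim input is held and the rotation is nearly aligned with it, FireShot spawns a projectile at FireLocation, throttled by a game-time fire-rate timer.
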(event EventBeginPlay)

(event Collision|EventActorBeginOverlap
  (params (OtherActor :type Actor%20Object%20Reference)))

(event EventTick
  (params (DeltaSeconds :type Float%20%28single-precision%29)))

(event Input|AxisEvents|InputAxisMoveHor
  (params (AxisValue :type Float%20%28single-precision%29))
  ;[1 1 1] Handle Movement
  (Pawn|Input|AddMovementInput "0.000000,1.000000, 0" AxisValue false))

(event Input|AxisEvents|InputAxisMoveVert
  (params (AxisValue :type Float%20%28single-precision%29))
  ;[1 1 1] Handle Movement
  (Pawn|Input|AddMovementInput "1.000000,0.000000, 0" AxisValue false))

(event Input|AxisEvents|InputAxisAimHor
  (params (AxisValue :type Float%20%28single-precision%29))
  (bind _returnvalue (Pawn|GetController))
  ;[1 1 1] Set rotation through smooth lerp based on looking Input
  (Pawn|SetControlRotation _returnvalue (Math|Rotator|Lerp(Rotator) (Pawn|GetControlRotation _returnvalue :!class /Script/Engine.Controller) (Math|Conversions|RotationFromXVector (Math|Vector|MakeVector (stale Input|AxisEvents|InputAxisAimVert AxisValue) AxisValue 0.0)) (* (Utilities|Time|GetWorldDeltaSeconds) (Variables|Default|GetTurnRate)) true))
  ;[1 1 1] If holding direction and fully looking in intended direction
  (if (and (Math|Rotator|Equal(Rotator) (Math|Conversions|RotationFromXVector (Math|Vector|MakeVector (stale Input|AxisEvents|InputAxisAimVert AxisValue) AxisValue 0.0)) (Pawn|GetControlRotation (Pawn|GetController) :!class /Script/Engine.Controller) 1e+01) (> (Math|Vector|VectorLength (Math|Vector|MakeVector (stale Input|AxisEvents|InputAxisAimVert AxisValue) AxisValue 0.0)) 0.0))
    (CallFunction|FireShot)))

(event Input|AxisEvents|InputAxisAimVert
  (params (AxisValue :type Float%20%28single-precision%29))
  (bind _returnvalue (Pawn|GetController))
  ;[1 1 1] Set rotation through smooth lerp based on looking Input
  (Pawn|SetControlRotation _returnvalue (Math|Rotator|Lerp(Rotator) (Pawn|GetControlRotation _returnvalue :!class /Script/Engine.Controller) (Math|Conversions|RotationFromXVector (Math|Vector|MakeVector AxisValue (stale Input|AxisEvents|InputAxisAimHor AxisValue) 0.0)) (* (Utilities|Time|GetWorldDeltaSeconds) (Variables|Default|GetTurnRate)) true))
  ;[1 1 1] If holding direction and fully looking in intended direction
  (if (and (Math|Rotator|Equal(Rotator) (Math|Conversions|RotationFromXVector (Math|Vector|MakeVector AxisValue (stale Input|AxisEvents|InputAxisAimHor AxisValue) 0.0)) (Pawn|GetControlRotation (Pawn|GetController) :!class /Script/Engine.Controller) 1e+01) (> (Math|Vector|VectorLength (Math|Vector|MakeVector AxisValue (stale Input|AxisEvents|InputAxisAimHor AxisValue) 0.0)) 0.0))
    (CallFunction|FireShot)))

(fn ConstructionScript)

(fn FireShot
  (bind _returnvalue (Utilities|Time|GetGameTimeinSeconds))
  ;[1 1 1] Fire Projectile
  (if (< (Variables|Default|GetFireTimer) _returnvalue)
    (Variables|Default|SetFireTimer (+ (Variables|Default|GetFireRate) _returnvalue))
    (Game|SpawnActorfromClass (Variables|Default|GetProjClass) (Transformation|GetWorldTransform (Variables|Default|GetFireLocation)) "AlwaysSpawn" 0 0)))