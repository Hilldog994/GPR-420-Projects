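; AI controller for a suicide-bomber enemy that chases the player and explodes on reaching them.
; On possess it caches the enemy pawn, and pawn sensing stores the first player character it sees and starts the chase.
; When the move succeeds, it deals full radial damage, spawns an explosion emitter and destroys the enemy.
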(event OnSeePawn(PawnSensing)
  (params (Pawn :type Pawn%20Object%20Reference))
  ;[1 1 1] Set player variable if it does not exist already
  (Variables|Default|GetPlayer
    (:then)
    (:else
      (bind _asbp_player_character (Utilities|Casting|CastToBP_PlayerCharacter Pawn))
      (Variables|Default|SetPlayer _asbp_player_character)
      (CallFunction|ChasePlayer))))

(event Custom|ChasePlayer
  (bind _enemy (Variables|Default|GetEnemy))
  (bind _returnvalue (Transformation|GetActorTransform _enemy))
  (bind (_location _rotation _scale) (Math|Transform|BreakTransform _returnvalue))
  (AI|AIMoveTo (Variables|Default|GetEnemy) "0, 0, 0" (Variables|Default|GetPlayer) 5e+01 true
    (:OnSuccess
      (Game|Damage|ApplyRadialDamage (Variables|Default|GetExplosionDamage) _location (Variables|Default|GetExplosionRadius) 0 0 _enemy 0 true "ECC_Visibility")
      (Effects|SpawnEmitteratLocation "/Game/StarterContent/Particles/P_Explosion.P_Explosion" _location _rotation _scale)
      (Actor|DestroyActor (Variables|Default|GetEnemy)))))

(event EventPossess
  (params (PossessedPawn :type Pawn%20Object%20Reference))
  (bind _asbp_enemy_base (Utilities|Casting|CastToBP_EnemyBase PossessedPawn))
  (Variables|Default|SetEnemy _asbp_enemy_base))

(fn ConstructionScript)