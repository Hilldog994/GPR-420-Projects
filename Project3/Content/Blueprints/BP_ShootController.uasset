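; BP_ShootController is an AI controller for the BP_Enemy_ShootPlayer enemy that tells it which player to target.
; On possession it caches the enemy pawn.
; Its AIPerception updates, filtered to BP_PlayerCharacter, store the sensed player and pass it to the enemy through SetPlayerTarget, or clear both when sensing is lost.
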(event OnTargetPerceptionUpdated(AIPerception)
  (params (Actor :type Actor%20Object%20Reference) (Stimulus :type AI%20Stimulus%20Structure))
  ;[1 1 1] Set player variable based on if they entered or left perception
  (bind _asbp_player_character (Utilities|Casting|CastToBP_PlayerCharacter Actor))
  (if (.bSuccessfullySensed (Utilities|Struct|BreakAIStimulus Stimulus))
    (bind _output_get (Variables|Default|SetPlayer _asbp_player_character))
    (Default|SetPlayerTarget (Variables|Default|GetEnemy) _output_get)
    (else
      (Variables|Default|SetPlayer 0)
      (Default|SetPlayerTarget (Variables|Default|GetEnemy)))))

(event EventPossess
  (params (PossessedPawn :type Pawn%20Object%20Reference))
  (bind _asbp_enemy_shoot_player (Utilities|Casting|CastToBP_Enemy_ShootPlayer PossessedPawn))
  (Variables|Default|SetEnemy _asbp_enemy_shoot_player))

(fn ConstructionScript)